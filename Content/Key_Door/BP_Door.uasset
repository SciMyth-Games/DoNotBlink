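; BP_Door is an interactable door that swings open once the player has inserted the required number of keys.
; An interaction sphere registers it as the player's current interactable and shows a prompt widget and UI message only while the player carries a key.
; Interact stores and destroys the carried key, then updates the player's progress and key UI.
; When the count is met, a timeline rotates the mesh's yaw.
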(event OnComponentBeginOverlap(InteractionSphere)
  (params (OverlappedComponent :type Primitive%20Component%20Object%20Reference) (OtherActor :type Actor%20Object%20Reference) (OtherComp :type Primitive%20Component%20Object%20Reference) (OtherBodyIndex :type Integer) (bFromSweep :type Boolean) (SweepResult :type Hit%20Result%20Structure%20%28by%20ref%29))
  (bind _playerref (Variables|Default|GetPLayerRef))
  (if (== OtherActor _playerref)
    (Variables|/Game/FirstPerson/Blueprints/BP_FirstPersonCharacter.BP_FirstPersonCharacter_C|SetCurrentInteractable _playerref self)
    (if (Utilities|IsValid (Variables|/Game/FirstPerson/Blueprints/BP_FirstPersonCharacter.BP_FirstPersonCharacter_C|GetCurrentKey _playerref))
      (Rendering|SetVisibility (Variables|Default|GetInteractionWidget) true false)
      (Class|BPIPlayer|SetInteractUI(Message) (Variables|Default|GetPLayerRef) true))))

(event OnComponentEndOverlap(InteractionSphere)
  (params (OverlappedComponent :type Primitive%20Component%20Object%20Reference) (OtherActor :type Actor%20Object%20Reference) (OtherComp :type Primitive%20Component%20Object%20Reference) (OtherBodyIndex :type Integer))
  (bind _playerref (Variables|Default|GetPLayerRef))
  (if (== OtherActor _playerref)
    (Variables|/Game/FirstPerson/Blueprints/BP_FirstPersonCharacter.BP_FirstPersonCharacter_C|SetCurrentInteractable _playerref 0)
    (Rendering|SetVisibility (Variables|Default|GetInteractionWidget) false false)
    (Class|BPIPlayer|SetInteractUI(Message) (Variables|Default|GetPLayerRef) false)))

(event Custom|OpenDoor
  (bind _doorrotation (Timeline|TL_OpenDoor Play)
    (:Update
      (Transformation|SetRelativeRotation (Variables|Default|GetStaticMesh) (Math|Rotator|MakeRotator 0.0 0.0 _doorrotation) false false))))

(event EventBeginPlay
  (Rendering|SetVisibility (Variables|Default|GetInteractionWidget) false false)
  (bind _asbp_first_person_character (Utilities|Casting|CastToBP_FirstPersonCharacter (Game|GetPlayerCharacter 0)))
  (bind _output_get (Variables|Default|SetPLayerRef _asbp_first_person_character))
  (Utilities|FlowControl|DelayUntilNextTick)
  (Default|UpdateDoorProgress _output_get (Utilities|Array|Length (Variables|Default|GetInsertedKeys)) (Variables|Default|GetRequiredKeys)))

(event Collision|EventActorBeginOverlap
  (params (OtherActor :type Actor%20Object%20Reference)))

(event EventTick
  (params (DeltaSeconds :type Float%20%28single-precision%29)))

(event EventInteract
  (params (Interactor :type Actor%20Object%20Reference))
  (bind _insertedkeys (Variables|Default|GetInsertedKeys))
  (bind _requiredkeys (Variables|Default|GetRequiredKeys))
  (bind _playerref (Variables|Default|GetPLayerRef))
  (bind _returnvalue (Utilities|Array|Length _insertedkeys))
  (if (== Interactor _playerref)
    (Utilities|IsValid (Variables|/Game/FirstPerson/Blueprints/BP_FirstPersonCharacter.BP_FirstPersonCharacter_C|GetCurrentKey _playerref)
      (:Is%20Valid
        (Rendering|SetVisibility (Variables|Default|GetInteractionWidget) false false)
        (Class|BPIPlayer|SetInteractUI(Message) (Variables|Default|GetPLayerRef) false)
        (Utilities|Array|AddUnique (Variables|Default|GetInsertedKeys) (Variables|/Game/FirstPerson/Blueprints/BP_FirstPersonCharacter.BP_FirstPersonCharacter_C|GetCurrentKey _playerref))
        (Actor|DestroyActor (Variables|/Game/FirstPerson/Blueprints/BP_FirstPersonCharacter.BP_FirstPersonCharacter_C|GetCurrentKey _playerref))
        (Variables|/Game/FirstPerson/Blueprints/BP_FirstPersonCharacter.BP_FirstPersonCharacter_C|SetCurrentKey _playerref 0)
        (Default|UpdateDoorProgress _playerref _returnvalue _requiredkeys)
        (Default|UpdateKeyUI _playerref)
        (if (>= _returnvalue _requiredkeys)
          (CallFunction|OpenDoor)
          (else
            (Development|PrintString "1/2 key received")))))))

(fn ConstructionScript)