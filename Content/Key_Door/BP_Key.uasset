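; BP_Key is a key pickup that the first-person character can take and carry in the right hand.
; Overlapping its InteractionSphere registers it as the character's current interactable and shows the prompt widget and UI message; leaving clears both.
; Interact works only if no valid key is held: it sets CurrentKey, updates key UI, snaps to the HandGrip_R socket, disables collision and hides the prompts.
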(event OnComponentBeginOverlap(InteractionSphere)
  (params (OverlappedComponent :type Primitive%20Component%20Object%20Reference) (OtherActor :type Actor%20Object%20Reference) (OtherComp :type Primitive%20Component%20Object%20Reference) (OtherBodyIndex :type Integer) (bFromSweep :type Boolean) (SweepResult :type Hit%20Result%20Structure%20%28by%20ref%29))
  (bind _asbp_first_person_character (Utilities|Casting|CastToBP_FirstPersonCharacter OtherActor))
  (Variables|/Game/FirstPerson/Blueprints/BP_FirstPersonCharacter.BP_FirstPersonCharacter_C|SetCurrentInteractable _asbp_first_person_character self)
  (Rendering|SetVisibility (Variables|Default|GetInteractionWidget) true false)
  (Class|BPIPlayer|SetInteractUI(Message) _asbp_first_person_character true))

(event OnComponentEndOverlap(InteractionSphere)
  (params (OverlappedComponent :type Primitive%20Component%20Object%20Reference) (OtherActor :type Actor%20Object%20Reference) (OtherComp :type Primitive%20Component%20Object%20Reference) (OtherBodyIndex :type Integer))
  (bind _asbp_first_person_character (Utilities|Casting|CastToBP_FirstPersonCharacter OtherActor))
  (Variables|/Game/FirstPerson/Blueprints/BP_FirstPersonCharacter.BP_FirstPersonCharacter_C|SetCurrentInteractable _asbp_first_person_character 0)
  (Rendering|SetVisibility (Variables|Default|GetInteractionWidget) false false)
  (Class|BPIPlayer|SetInteractUI(Message) _asbp_first_person_character false))

(event EventBeginPlay
  (Rendering|SetVisibility (Variables|Default|GetInteractionWidget) false false))

(event Collision|EventActorBeginOverlap
  (params (OtherActor :type Actor%20Object%20Reference)))

(event EventTick
  (params (DeltaSeconds :type Float%20%28single-precision%29)))

(event EventInteract
  (params (Interactor :type Actor%20Object%20Reference))
  (bind _asbp_first_person_character (Utilities|Casting|CastToBP_FirstPersonCharacter Interactor))
  (if (not (Utilities|IsValid (Variables|/Game/FirstPerson/Blueprints/BP_FirstPersonCharacter.BP_FirstPersonCharacter_C|GetCurrentKey _asbp_first_person_character)))
    (Variables|/Game/FirstPerson/Blueprints/BP_FirstPersonCharacter.BP_FirstPersonCharacter_C|SetCurrentKey _asbp_first_person_character self)
    (Default|UpdateKeyUI _asbp_first_person_character)
    (Transformation|AttachComponentToComponent (Variables|/Game/FirstPerson/Blueprints/BP_FirstPersonCharacter.BP_FirstPersonCharacter_C|GetFirstPersonMesh _asbp_first_person_character) "HandGrip_R" "SnapToTarget" "SnapToTarget" "KeepWorld" true)
    (Collision|SetActorEnableCollision false)
    (Development|PrintString "\"Picked Up Key\"")
    (Rendering|SetVisibility (Variables|Default|GetInteractionWidget) false false)
    (Class|BPIPlayer|SetInteractUI(Message) _asbp_first_person_character false)))

(fn ConstructionScript)