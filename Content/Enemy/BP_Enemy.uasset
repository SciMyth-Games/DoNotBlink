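; Enemy character that freezes while the player looks at it and chases them while unobserved.
; First sighting by PawnSensing starts a looping timer that tests visibility with a camera-forward dot product and a line trace to the head socket.
; Each check either stops movement or starts an AI MoveTo toward the player.
; Overlapping the kill sphere plays an attack montage, whose notify is meant to kill the player if still within range.
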(event OnComponentBeginOverlap(KillSphere)
  (params (OverlappedComponent :type Primitive%20Component%20Object%20Reference) (OtherActor :type Actor%20Object%20Reference) (OtherComp :type Primitive%20Component%20Object%20Reference) (OtherBodyIndex :type Integer) (bFromSweep :type Boolean) (SweepResult :type Hit%20Result%20Structure%20%28by%20ref%29))
  (if (== OtherActor (Variables|Default|GetPlayerRef))
    (Variables|Default|SetCurrentState "NewEnumerator3")
    (bind _notifyname (Animation|Montage|PlayMontage (Variables|Character|GetMesh) "/Game/Characters/Mannequins/Anims/Unarmed/Attack/MM_Attack.MM_Attack")
      (:then
        (Variables|Default|SetCurrentState "NewEnumerator0" :!label _label))
      (:OnCompleted
        (goto _label))
      (:OnNotifyBegin
        (if (== _notifyname "AttackHit")
          (if (<= (Transformation|GetDistanceTo self (Variables|Default|GetPlayerRef)) 1e+02)
            (Default|PlayerDeath (Variables|Default|GetPlayerRef))
            (Development|PrintString "Player Dead")
            (else
              (Development|PrintString "Player Escaped"))))))))

(event OnSeePawn(PawnSensing)
  (params (Pawn :type Pawn%20Object%20Reference))
  (if (not (Variables|Default|GetHasBeenDiscovered))
    (Variables|Default|SetHasBeenDiscovered true)
    (Variables|Default|SetCurrentState "NewEnumerator0")
    (Utilities|Time|SetTimerbyFunctionName 0 "CheckVisibility" (Variables|Default|GetVisibilityUpdateRate) true)))

(event Custom|UpdateMovementState
  (if (Variables|Default|GetIsVisibleToPlayer)
    (AI|Navigation|StopMovement (Pawn|GetController))
    (Variables|Default|SetCurrentState "NewEnumerator0")
    (elif (Utilities|Enum|NotEqual(Enum) (Variables|Default|GetCurrentState) "NewEnumerator1")
      (AI|AIMoveTo self "0, 0, 0" (Variables|Default|GetPlayerRef) 15.0 false
        (:then
          (Variables|Default|SetCurrentState "NewEnumerator1"))))))

(event EventBeginPlay
  (bind _asbp_first_person_character (Utilities|Casting|CastToBP_FirstPersonCharacter (Game|GetPlayerCharacter 0)))
  (Variables|Default|SetPlayerRef _asbp_first_person_character))

(event EventTick
  (params (DeltaSeconds :type Float%20%28single-precision%29))
  (Development|PrintString (Utilities|String|ToString(Boolean) (Variables|Default|GetIsVisibleToPlayer)) true true "(R=0.000000,G=0.660000,B=1.000000,A=1.000000)" 2.0 "1None"))

(fn ConstructionScript)

(fn CheckVisibility
  (bind _playerref (Variables|Default|GetPlayerRef))
  (bind _firstpersoncamera (Variables|/Game/FirstPerson/Blueprints/BP_FirstPersonCharacter.BP_FirstPersonCharacter_C|GetFirstPersonCamera _playerref))
  (bind _returnvalue (Transformation|GetWorldLocation _firstpersoncamera))
  (Utilities|IsValid (Variables|Default|GetPlayerRef)
    (:Is%20Valid
      (if (> (Math|Vector|DotProduct (Math|Vector|GetForwardVector _firstpersoncamera) (Math|Vector|Normalize (- (Transformation|GetActorLocation) _returnvalue))) 0.7)
        (bind _returnvalue_2 (Collision|LineTraceByChannel _returnvalue (Transformation|GetSocketLocation (Variables|Character|GetMesh) "head") "TraceTypeQuery1" false 0 "ForDuration"))
        (Variables|Default|SetIsVisibleToPlayer (not _returnvalue_2))
        (CallFunction|UpdateMovementState)
        (else
          (Variables|Default|SetIsVisibleToPlayer false)
          (CallFunction|UpdateMovementState))))))

(fn SetWatched
  (params (Watched :type Boolean))
  (Variables|Default|SetIsVisibleToPlayer Watched))